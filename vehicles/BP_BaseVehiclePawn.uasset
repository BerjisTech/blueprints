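; Base Chaos vehicle pawn that assembles a modular car from data tables, with openable doors and swappable mods.
; SetUpBody applies a DT_VehicleSetup row to skeleton, rims, wheels (radius from mesh bounds) and socket-attached body parts, then loads DT_ModPresets mods.
; Mod selection replaces the component sharing the key's "~" suffix, while key substrings frame the spring-arm camera.
; Timelines swing doors, and SideLights mods flash by endlessly rotating material slots.
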(event Custom|setUpBody
  (Utilities|ResetBody)
  (bind _returnvalue (Utilities|GetDataTableRow "/Game/Blueprints/tables/DT_VehicleSetup.DT_VehicleSetup" (Variables|Mods|GetBody%20Meshes%20Row))
    (:then
      (Components|SkeletalMesh|SetSkeletalMeshAsset (Variables|Character|GetMesh) (.skeletalmesh _returnvalue))
      (Class|SkeletalMeshComponent|SetAnimClass (Variables|Character|GetMesh) (.animationclass _returnvalue))
      (CallFunction|SetUpRims (.rims _returnvalue))
      (CallFunction|SetUpWheels (.wheels _returnvalue))
      (Components|StaticMesh|SetStaticMesh (Variables|Default|GetBody) (.bodymesh _returnvalue))
      (for _array_element (Variables|Default|GetattachedParts)
        (Components|DestroyComponent _array_element))
      (CallFunction|AddBodyMeshes (.bodymeshattachemnts _returnvalue))
      (CallFunction|LoadMods)
      (CallFunction|SetUpDoors (.doors _returnvalue) (.doorwindows _returnvalue)))))

(event Custom|loadMods
  (CallFunction|LoadDefaultMods)
  (CallFunction|LoadModsClient))

(event Custom|openDoor
  (params (door :type Static%20Mesh%20Component%20Object%20Reference))
  (Utilities|IsValid door
    (:Is%20Valid
      (bind _zrotate (Timeline|openTheDoor Play)
        (:Update
          (Transformation|SetRelativeRotation door (Math|Rotator|MakeRotator 0.0 0.0 _zrotate) false false))))))

(event Custom|closeDoor
  (params (door :type Static%20Mesh%20Component%20Object%20Reference))
  (Utilities|IsValid door
    (:Is%20Valid
      (bind _zrotate (Timeline|closeTheDoor Play)
        (:Update
          (Transformation|SetRelativeRotation door (Math|Rotator|MakeRotator 0.0 0.0 _zrotate) false false))))))

(event Custom|rotateMaterials
  (params (component :type Static%20Mesh%20Component%20Object%20Reference))
  (bind _returnvalue (Rendering|Material|GetNumMaterials component))
  (bind _returnvalue_2 (- _returnvalue 1))
  (for _index (range 0 _returnvalue_2) :!label _label
    (if (== _index 0)
      (Variables|Default|SetFirstMaterial (Rendering|Material|GetMaterial component _index)))
    (Rendering|Material|SetMaterial component _index (select (== _index _returnvalue_2) (Variables|Default|GetFirstMaterial) (Rendering|Material|GetMaterial component (Math|Integer|%(Integer) (+ _index 1) _returnvalue)))))
  (Utilities|FlowControl|Delay 0.2)
  (goto _label))

(event Custom|openDoorServer
  (params (door :type Static%20Mesh%20Component%20Object%20Reference))
  (CallFunction|OpenDoor door))

(event Custom|close%20door%20server
  (params (door :type Static%20Mesh%20Component%20Object%20Reference))
  (CallFunction|CloseDoor door))

(event Custom|loadModsClient
  (EventDispatchers|BindEventtoUpdateVehicleMod (EventDispatchers|CreateEvent :!event Custom|displayMods)))

(event Custom|displayMods
  (params (modKey :type Name))
  (bind _returnvalue (Utilities|String|ToString(Name) modKey))
  (bind _mods (Variables|Mods|Getmods))
  (bind _rights (Utilities|String|Split _returnvalue "~"))
  (bind _returnvalue_2 (Utilities|String|StringToName _rights))
  (bind (_value _returnvalue_3) (Utilities|Map|Find _mods _returnvalue_2))
  (if _returnvalue_3
    (Components|DestroyComponent _value))
  (Utilities|AddModComponentandMesh (.Value (Utilities|Map|Find (Variables|Mods|GetSelectableModsMesh) modKey)) _rights))

(event Custom|load%20default%20mods
  (bind _returnvalue (Utilities|GetDataTableRow "/Game/Blueprints/tables/DT_ModPresets.DT_ModPresets" (Variables|Mods|GetModPreset))
    (:then
      (bind _keys (Utilities|Map|Keys (.modmeshes _returnvalue)))
      (for _array_element _keys
        (Utilities|AddModComponentandMesh (.Value (Utilities|Map|Find (.modmeshes _returnvalue) _array_element)) (Utilities|String|ToString(Name) _array_element))))))

(event Custom|setUpRims
  (params (rimAssets :type Map%20of%20Names%20to%20Objects))
  (for _index (range 0 (- (Utilities|Map|Length rimAssets) 1))
    (Components|StaticMesh|SetStaticMesh (Utilities|Select :Index _index :Option%200 (Variables|Default|GetFL) :Option%201 (Variables|Default|GetFR) :Option%202 (Variables|Default|GetRL) :Option%203 (Variables|Default|GetRR)) (.Value (Utilities|Map|Find rimAssets (Transformation|GetAttachSocketName (Utilities|Select :Index _index :Option%200 (Variables|Default|GetFL) :Option%201 (Variables|Default|GetFR) :Option%202 (Variables|Default|GetRL) :Option%203 (Variables|Default|GetRR))))))))

(event Custom|setUpWheels
  (params (wheelAssets :type Map%20of%20Names%20to%20Objects))
  (for _index (range 0 (- (Utilities|Map|Length wheelAssets) 1))
    (Utilities|IsValid (.Value (Utilities|Map|Find wheelAssets (Utilities|Select :Index _index :Option%200 "FL" :Option%201 "FR" :Option%202 "RL" :Option%203 "RR")))
      (:Is%20Valid
        (Components|StaticMesh|SetStaticMesh (Utilities|Select :Index _index :Option%200 (Variables|Default|GetwFL) :Option%201 (Variables|Default|GetwFR) :Option%202 (Variables|Default|GetwRL) :Option%203 (Variables|Default|GetwRR)) (.Value (Utilities|Map|Find wheelAssets (Utilities|Select :Index _index :Option%200 "FL" :Option%201 "FR" :Option%202 "RL" :Option%203 "RR"))))
        (Class|ChaosWheeledVehicleMovementComponent|SetWheelRadius (.AsChaos%20Wheeled%20Vehicle%20Movement%20Component (Utilities|Casting|CastToChaosWheeledVehicleMovementComponent (Variables|Default|GetVehicleMovementComponent))) _index (.sphereradius (StaticMesh|GetBounds (.Value (Utilities|Map|Find wheelAssets (Utilities|Select :Index _index :Option%200 "FL" :Option%201 "FR" :Option%202 "RL" :Option%203 "RR"))))))))))

(event Custom|addBodyMeshes
  (params (mesh :type Array%20of%20Static%20Mesh%20Object%20References))
  (for _array_element mesh
    (Utilities|AddBodyComponent "root" _array_element false)))

(event Custom|setUpDoors
  (params (doors :type Map%20of%20Names%20to%20Objects) (doorWindows :type Map%20of%20Names%20to%20Objects))
  (bind _keys (Utilities|Map|Keys doors))
  (for _array_element _keys
    (Utilities|AddBodyComponent _array_element (.Value (Utilities|Map|Find doors _array_element)) true))
  (bind _keys_2 (Utilities|Map|Keys doorWindows))
  (for _array_element_2 _keys_2
    (Utilities|AddBodyComponent _array_element_2 (.Value (Utilities|Map|Find doorWindows _array_element_2)) false)))

(event Custom|exitModMenu
  (EventDispatchers|BindEventtoResetCamera (EventDispatchers|CreateEvent :!event Custom|restCameraAfterModding)))

(event Custom|removeStaticMeshes
  (Components|DestroyComponent (Actor|GetComponentsByClass "/Script/Engine.StaticMeshComponent")))

(event Custom|updateCameraPosition
  (params (cameraPositionKey :type Name))
  (bind _returnvalue (Utilities|String|ToString(Name) cameraPositionKey))
  (bind _backspringarm (Variables|Default|GetBackSpringArm))
  (bind _backspringarm_2 (Variables|Default|GetBackSpringArm))
  (bind _backspringarm_3 (Variables|Default|GetBackSpringArm))
  (bind _backspringarm_4 (Variables|Default|GetBackSpringArm))
  (bind _returnvalue_2 (Utilities|String|Contains _returnvalue "rim"))
  (bind _returnvalue_3 (Utilities|String|Contains _returnvalue "seats"))
  (bind _returnvalue_4 (Utilities|String|Contains _returnvalue "interiors"))
  (bind _relativerotation (Variables|/Script/Engine.SceneComponent|GetRelativeRotation _backspringarm_2))
  (bind _relativerotation_2 (Variables|/Script/Engine.SceneComponent|GetRelativeRotation _backspringarm_3))
  (bind _relativerotation_3 (Variables|/Script/Engine.SceneComponent|GetRelativeRotation _backspringarm_4))
  (bind _relativerotation_4 (Variables|/Script/Engine.SceneComponent|GetRelativeRotation _backspringarm))
  (bind _returnvalue_5 (or _returnvalue_4 _returnvalue_3))
  (if (Utilities|String|Contains _returnvalue "front")
    (Transformation|SetRelativeRotation _backspringarm_3 (Math|Rotator|MakeRotator (.roll _relativerotation_2) (.pitch _relativerotation_2) 1.8e+02) false false))
  (if (Utilities|String|Contains _returnvalue "back")
    (Transformation|SetRelativeRotation _backspringarm (Math|Rotator|MakeRotator (.roll _relativerotation_4) (.pitch _relativerotation_4) 0.0) false false))
  (if (or (Utilities|String|Contains _returnvalue "side") _returnvalue_2)
    (Transformation|SetRelativeRotation _backspringarm_4 (Math|Rotator|MakeRotator (.roll _relativerotation_3) (.pitch _relativerotation_3) 9e+01) false false))
  (Variables|/Script/Engine.SpringArmComponent|SetSocketOffset (Variables|Default|GetBackSpringArm) (Math|Vector|SelectVector "0, 0, 0" "0.000000,0.000000,300.000000" (or _returnvalue_2 (Utilities|String|Contains _returnvalue "bumper"))))
  (if _returnvalue_5
    (Transformation|SetRelativeRotation _backspringarm_2 (Math|Rotator|MakeRotator (.roll _relativerotation) (.pitch _relativerotation) 0.0) false false)
    (Variables|/Script/Engine.SpringArmComponent|SetSocketOffset _backspringarm_2 "0.000000,0.000000,150.000000"))
  (Variables|/Script/Engine.SpringArmComponent|SetTargetArmLength _backspringarm_2 (Math|Float|SelectFloat 3e+02 9e+02 _returnvalue_5))
  (Variables|/Script/Engine.SpringArmComponent|SetbDoCollisionTest _backspringarm_2 (not _returnvalue_5)))

(event Custom|restCameraAfterModding
  (bind _backspringarm (Variables|Default|GetBackSpringArm))
  (Variables|/Script/Engine.SpringArmComponent|SetSocketOffset _backspringarm "0.000000,0.000000,300.000000")
  (Variables|/Script/Engine.SpringArmComponent|SetTargetArmLength _backspringarm 9e+02)
  (Transformation|SetRelativeRotation _backspringarm (Math|Interpolation|RInterpTo (Variables|/Script/Engine.SceneComponent|GetRelativeRotation _backspringarm) "0, 0, 0" (Utilities|Time|GetWorldDeltaSeconds) 1.0) false false))

(event EventBeginPlay
  (CallFunction|SetUpBody))

(event Collision|EventActorBeginOverlap
  (params (OtherActor :type Actor%20Object%20Reference)))

(event EventTick
  (params (DeltaSeconds :type Float%20%28single-precision%29)))

(fn ConstructionScript)

(fn GetBodySocketLoaction
  (params (InSocketName :type Name))
  (return (Transformation|GetSocketLocation (Variables|Default|GetBody) InSocketName)))