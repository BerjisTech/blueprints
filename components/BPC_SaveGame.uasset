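; Player save-game component that persists the player's last location and restores it when play begins.
; On BeginPlay it loads or creates the SG_PlayerData slot and registers it with SomboGameInstance.
; It teleports the pawn to a landscape trace from the saved location, or from PlayerStart if that is zero.
; Self-repeating short-delay loops continually record location and asynchronously rewrite the slot.
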(event Custom|updatePlayerLocation
  (bind _sg_player_data (Variables|Default|GetSG%20Player%20Data))
  (Utilities|IsValid _sg_player_data
    (:Is%20Valid
      (Variables|/Game/Blueprints/game_save/SG_PlayerData.SG_PlayerData_C|SetlastLocation _sg_player_data (Transformation|GetActorLocation (Game|Player|GetPlayerPawn 0))))
    (:Is%20Not%20Valid
      _))
  (Utilities|FlowControl|Delay 0.0002)
  (CallFunction|UpdatePlayerLocation))

(event Custom|saveGame
  (bind _sg_player_data (Variables|Default|GetSG%20Player%20Data))
  (Utilities|IsValid _sg_player_data
    (:Is%20Valid
      (|AsyncSaveGametoSlot _sg_player_data (Variables|Default|GetSlot%20Name)
        (:Completed
          (Variables|/Game/Blueprints/GameMode/SomboGameInstance.SomboGameInstance_C|SetcurrentGame (Variables|Default|GetgameInstance) (Variables|Default|GetSG%20Player%20Data))
          (Utilities|FlowControl|Delay 0.0002)
          (CallFunction|SaveGame))))))

(event Custom|loadPlayerDetailsFromSettings
  (bind _returnvalue (Game|GetPlayerCharacter 0))
  (bind _sg_player_data (Variables|Default|GetSG%20Player%20Data))
  (bind _capsulecomponent (Variables|/Script/Engine.Character|GetCapsuleComponent _returnvalue))
  (bind _lastlocation (Variables|/Game/Blueprints/game_save/SG_PlayerData.SG_PlayerData_C|GetlastLocation _sg_player_data))
  (bind _returnvalue_2 (Actor|GetActorOfClass "/Script/Engine.PlayerStart"))
  (bind _array_element_impact_point (CallFunction|LineTraceforLandscape (select (Class|KismetMathLibrary|EqualExactlyVectorVector _lastlocation "0, 0, 0") (Transformation|GetActorLocation _returnvalue_2) _lastlocation) "0.000000,0.000000,-1000000.000000"))
  (Transformation|SetActorLocation (Game|Player|GetPlayerPawn 0) _array_element_impact_point false true)
  (Class|PrimitiveComponent|SetPhysicsAngularVelocityinDegrees _capsulecomponent "0, 0, 0" false "None")
  (Physics|SetPhysicsLinearVelocity _capsulecomponent "0, 0, 0" false "None"))

(event Custom|setUpOwner
  (bind _returnvalue (Components|GetOwner))
  (Variables|Default|SetgameInstance (.AsSombo%20Game%20Instance (Utilities|Casting|CastToSomboGameInstance (Game|GetGameInstance))))
  (Variables|Default|SetSlot%20Name (Variables|Default|GetSlot%20Name))
  (bind _output_get (Variables|Default|Setowner _returnvalue))
  (bind _ascharacter (Utilities|Casting|CastToCharacter _output_get)
    (:then
      (Variables|Default|SetCharacter _ascharacter)
      (bind _output_get_2 (Variables|Default|SetcharacterController (Pawn|GetController (Variables|/Script/Engine.Actor|GetInstigator _returnvalue)))))
    (:CastFailed
      _))
  (bind _asplayer_controller (Utilities|Casting|CastToPlayerController _output_get_2))
  (bind _output_get_3 (Variables|Default|SetPlayer%20Controller _asplayer_controller))
  (Variables|Default|SetControlled%20Pawn (Pawn|GetControlledPawn _output_get_3))
  (Variables|/Game/Blueprints/GameMode/SomboGameInstance.SomboGameInstance_C|SetsaveGame (Variables|Default|GetgameInstance) self)
  (Variables|/Game/Blueprints/GameMode/SomboGameInstance.SomboGameInstance_C|SetcurrentGame (Variables|Default|GetgameInstance) (Variables|Default|GetSG%20Player%20Data)))

(event Custom|serverSync
  (CallFunction|SetUpOwner)
  (bind _returnvalue (SaveGame|DoesSaveGameExist (Variables|Default|GetSlot%20Name)))
  (if _returnvalue
    (Utilities|LoadGame)
    (else
      (Utilities|CreateGame)))
  (CallFunction|LoadPlayerDetailsfromSettings)
  (CallFunction|SaveGame)
  (CallFunction|UpdatePlayerLocation))

(event EventBeginPlay
  (CallFunction|ServerSync))

(event EventTick
  (params (DeltaSeconds :type Float%20%28single-precision%29)))

(event EventVehiclePossesed
  (params (possedVehicle :type Wheeled%20Vehicle%20Pawn%20Soft%20Object%20Reference)))

(event EventTakeDamage)

(fn SpawnVehiclenearby
  (return false))