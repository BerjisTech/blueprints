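; BPC_UI_Manager handles hotkey-driven UI, toggling QuickActions with M and PauseMenu with P through a shared helper that creates or removes widgets and switches cursor and input mode.
; Escape uses a FlipFlop to open and close PauseMenu, faking pause with near-zero time dilation; OnKeyDown also opens it.
; Holding F speeds up game time and boosts player jump and walk speed.
; FastTravelWidget and Phone toggles are unwired.
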(event Custom|PauseMenu
  (bind _returnvalue (Game|GetPlayerController 0))
  (bind _returnvalue_2 (UserInterface|CreateWidget "/Game/Blueprints/widgets/PauseMenu.PauseMenu_C"))
  (UserInterface|Viewport|AddtoViewport _returnvalue_2 0)
  (Variables|/Script/Engine.PlayerController|SetbShowMouseCursor _returnvalue true)
  (Input|SetInputModeGameandUI _returnvalue _returnvalue_2 "LockAlways" true true)
  (Utilities|Time|SetGlobalTimeDilation 0.01))

(event EventTick
  (params (DeltaSeconds :type Float%20%28single-precision%29)))

(event Input|KeyboardEvents|M
  (params (Key :type Key%20Structure :default "None"))
  (:Pressed
    (Utilities|GameandUIWidgets "/Game/Blueprints/widgets/QuickActions.QuickActions_C")))

(event Input|KeyboardEvents|P
  (params (Key :type Key%20Structure :default "None"))
  (:Pressed
    (Utilities|GameandUIWidgets "/Game/Blueprints/widgets/PauseMenu.PauseMenu_C")))

(event Input|KeyboardEvents|Escape
  (params (Key :type Key%20Structure :default "None"))
  (bind _returnvalue (Game|GetPlayerController 0))
  (:Pressed
    (Utilities|FlowControl|FlipFlop
      (:A
        (bind _returnvalue_2 (UserInterface|CreateWidget "/Game/Blueprints/widgets/PauseMenu.PauseMenu_C"))
        (UserInterface|Viewport|AddtoViewport _returnvalue_2 0)
        (Variables|/Script/Engine.PlayerController|SetbShowMouseCursor _returnvalue true)
        (Input|SetInputModeGameandUI _returnvalue _returnvalue_2 "LockAlways" true true)
        (Utilities|Time|SetGlobalTimeDilation 0.01))
      (:B
        (bind _foundwidgets (Widget|GetAllWidgetsOfClass "/Game/Blueprints/widgets/PauseMenu.PauseMenu_C" true))
        (Widget|RemovefromParent _foundwidgets)
        (Variables|/Script/Engine.PlayerController|SetbShowMouseCursor _returnvalue false)
        (Input|SetInputModeGameOnly _returnvalue true)
        (Game|SetGamePaused false)
        (Utilities|Time|SetGlobalTimeDilation 1.0)))))

(event Input|KeyboardEvents|F
  (params (Key :type Key%20Structure :default "None"))
  (bind _returnvalue (Game|GetPlayerCharacter 0))
  (bind _charactermovement (Variables|/Script/Engine.Character|GetCharacterMovement _returnvalue))
  (:Pressed
    (Utilities|Time|SetGlobalTimeDilation 1e+01)
    (Utilities|IsValid _returnvalue
      (:Is%20Valid
        (Variables|/Script/Engine.CharacterMovementComponent|SetJumpZVelocity _charactermovement 1.2e+04)
        (Variables|/Script/Engine.CharacterMovementComponent|SetMaxWalkSpeed _charactermovement 1.2e+04))))
  (:Released
    (Utilities|Time|SetGlobalTimeDilation 1.0)
    (Utilities|IsValid 0
      (:Is%20Valid
        (Variables|/Script/Engine.CharacterMovementComponent|SetJumpZVelocity _charactermovement 6e+02)
        (Variables|/Script/Engine.CharacterMovementComponent|SetMaxWalkSpeed _charactermovement 6e+02)))))

(fn OnKeyDown
  (params (MyGeometry :type Geometry%20Structure) (InKeyEvent :type Key%20Event%20Structure))
  (if (== (Class|KismetInputLibrary|GetKey InKeyEvent) "Escape")
    (CallFunction|PauseMenu)
    (return (Class|WidgetBlueprintLibrary|Handled))
    (else
      (return (Class|WidgetBlueprintLibrary|Unhandled)))))