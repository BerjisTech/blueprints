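; Player character component that handles Enhanced Input movement, position reset and getting into vehicles.
; On interact it finds a nearby wheeled vehicle or spawns one, then repeatedly moves the character toward the driver door socket.
; It handles the door, delegates possession to BPC_VehicleInteraction and hides the character by scaling it to zero.
; It also attaches BPC_SaveGame, pushes hit meshes with impulses, swaps character meshes and destroys stored vehicles.
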(event Custom|findVehicle)

(event Custom|scalePlayer
  (bind _character (Variables|Default|Getcharacter))
  (bind _returnvalue (Transformation|GetActorTransform _character))
  (Transformation|SetActorTransform _character (Math|Transform|MakeTransform (.location _returnvalue) (.rotation _returnvalue) "0.000000,0.000000,0.000000") false true))

(event Custom|ApplyForceOnHit
  (Collision|AssignOnActorHit (Variables|Default|Getcharacter) (delegate Custom|OnActorHit_Event)))

(event Custom|customizeCharacter
  (params (character :type STRUCT%20Characters%20Structure))
  (bind _ascharacter (Utilities|Casting|CastToCharacter (Components|GetOwner)))
  (Components|SkeletalMesh|SetSkeletalMeshAsset (Variables|/Script/Engine.Character|GetMesh _ascharacter) (.skeletalmesh character)))

(event Custom|OnActorHit_Event
  (params (SelfActor :type Actor%20Object%20Reference) (OtherActor :type Actor%20Object%20Reference) (NormalImpulse :type Vector) (Hit :type Hit%20Result%20Structure%20%28by%20ref%29))
  (bind _returnvalue (Actor|GetComponentbyClass OtherActor "/Script/Engine.StaticMeshComponent"))
  (Utilities|IsValid _returnvalue
    (:Is%20Valid
      (Physics|AddImpulse _returnvalue (* NormalImpulse 2e+01) "None" false))))

(event Custom|returnVehicleToStorage_1
  (bind _vehicle (Variables|Default|GetVehicle))
  (Utilities|IsValid _vehicle
    (:Is%20Valid
      (Actor|DestroyActor _vehicle)
      (bind _assombo_game_instance (Utilities|Casting|CastToSomboGameInstance (Game|GetGameInstance)))
      (Variables|/Game/Blueprints/game_save/SG_PlayerData.SG_PlayerData_C|Setactivevehicle (Variables|/Game/Blueprints/GameMode/SomboGameInstance.SomboGameInstance_C|GetcurrentGame _assombo_game_instance) ""))))

(event Input|EnhancedActionEvents|EnhancedInputActionIA_Jump
  (params (ActionValue :type Boolean) (ElapsedSeconds :type Float%20%28double-precision%29) (TriggeredSeconds :type Float%20%28double-precision%29) (InputAction :type Input%20Action%20Object%20Reference :default "/Game/Blueprints/Input/Actions/IA_Jump.IA_Jump"))
  (bind _character (Variables|Default|Getcharacter))
  (:Started
    (Character|Jump _character))
  (:Completed
    (Character|StopJumping _character)))

(event Input|EnhancedActionEvents|EnhancedInputActionIA_Move
  (params (ActionValue :type Vector%202D%20Structure) (ElapsedSeconds :type Float%20%28double-precision%29) (TriggeredSeconds :type Float%20%28double-precision%29) (InputAction :type Input%20Action%20Object%20Reference :default "/Game/Blueprints/Input/Actions/IA_Move.IA_Move"))
  (bind _character (Variables|Default|Getcharacter))
  (bind _returnvalue (Pawn|GetControlRotation _character :!class /Script/Engine.Pawn))
  (Pawn|Input|AddMovementInput _character (Math|Vector|GetRightVector (Math|Rotator|MakeRotator (.roll _returnvalue) 0.0 (.yaw _returnvalue))) (.x ActionValue) false)
  (Pawn|Input|AddMovementInput _character (Math|Vector|GetForwardVector (Math|Rotator|MakeRotator 0.0 0.0 (.yaw (Pawn|GetControlRotation _character :!class /Script/Engine.Pawn)))) (.y ActionValue) false))

(event Input|EnhancedActionEvents|EnhancedInputActionIA_Reset
  (params (ActionValue :type Boolean) (ElapsedSeconds :type Float%20%28double-precision%29) (TriggeredSeconds :type Float%20%28double-precision%29) (InputAction :type Input%20Action%20Object%20Reference :default "/Game/Blueprints/Input/Actions/IA_Reset.IA_Reset"))
  (bind _returnvalue (Game|Player|GetPlayerPawn 0))
  (bind _returnvalue_2 (Components|GetOwner))
  (bind _returnvalue_3 (Transformation|GetActorLocation _returnvalue))
  (bind _outactors (Actor|GetAllActorsOfClass "/Script/Engine.PlayerStart"))
  (if (not (> (CallFunction|DistancetoKilometers (.Distance (Actor|FindNearestActor _returnvalue_3 _outactors))) 2e+01))
    (Transformation|SetActorLocation _returnvalue_2 (select (> (CallFunction|DistancetoKilometers (Math|Vector|Distance(Vector) (Transformation|GetActorLocation (.OutItem (Utilities|Array|Random _outactors))) _returnvalue_3)) 2e+01) _returnvalue_3 (Transformation|GetActorLocation (.OutItem (Utilities|Array|Random _outactors)))) false true)
    (CallFunction|AligntoLandscape _returnvalue_2)))

(event Input|EnhancedActionEvents|EnhancedInputActionIA_Look
  (params (ActionValue :type Vector%202D%20Structure) (ElapsedSeconds :type Float%20%28double-precision%29) (TriggeredSeconds :type Float%20%28double-precision%29) (InputAction :type Input%20Action%20Object%20Reference :default "/Game/Blueprints/Input/Actions/IA_Look.IA_Look"))
  (bind _character (Variables|Default|Getcharacter))
  (Pawn|Input|AddControllerYawInput _character (.x ActionValue))
  (Pawn|Input|AddControllerPitchInput _character (.y ActionValue)))

(event Input|EnhancedActionEvents|EnhancedInputActionIA_Interact
  (params (ActionValue :type Boolean) (ElapsedSeconds :type Float%20%28double-precision%29) (TriggeredSeconds :type Float%20%28double-precision%29) (InputAction :type Input%20Action%20Object%20Reference :default "/Game/Blueprints/Input/Actions/IA_Interact.IA_Interact"))
  (:Started
    (bind _aswheeled_vehicle_pawn (Utilities|FindNearbyVehicle)
      (:no%20vehicle%20found
        (Utilities|SpawnNewVehicle :!label _label))
      (:Found
        (Variables|Default|SetVehicle _aswheeled_vehicle_pawn))
      (:Vehicles%20Too%20Far%20Away
        (goto _label)))
    (Utilities|AddInteractionComponent (Variables|Default|GetVehicle) "/Game/Blueprints/components/BPC_VehicleInteraction.BPC_VehicleInteraction_C"
      (:Found%20Component
        _)
      (:addedComponent
        _))
    (Utilities|MovePlayertoVehicle (Variables|Default|GetVehicle)
      (:then
        (Utilities|HandleDoorsandPossesVehicle :!label _label_2))
      (:CastFailed
        (goto _label_2 directPosses)))))

(event EventBeginPlay
  (bind _ascharacter (Utilities|Casting|CastToCharacter (Components|GetOwner)))
  (bind _output_get (Variables|Default|Setcharacter _ascharacter))
  (bind _asplayer_controller (Utilities|Casting|CastToPlayerController (Pawn|GetController _output_get)))
  (Variables|Default|SetPlayer%20Controller _asplayer_controller)
  (Input|AddMappingContext (PlayerController|LocalPlayerSubsystems|GetEnhancedInputLocalPlayerSubsystem _asplayer_controller) "/Game/Blueprints/Input/IMC_OWT.IMC_OWT" 1 "(bIgnoreAllPressedKeysUntilRelease=True,bForceImmediately=False,bNotifyUserSettings=False)")
  (Utilities|AddInteractionComponent (Variables|Default|Getcharacter) "/Game/Blueprints/components/BPC_SaveGame.BPC_SaveGame_C"
    (:Found%20Component
      _)
    (:addedComponent
      _))
  (CallFunction|ApplyForceonHit))

(event EventTick
  (params (DeltaSeconds :type Float%20%28single-precision%29)))

(event EventPossessVehicle
  (params (possess :type Boolean) (is_npc :type Boolean) (vehicle :type Wheeled%20Vehicle%20Pawn%20Soft%20Object%20Reference) (driver :type Character%20Soft%20Object%20Reference))
  (bind _output_get (Variables|Default|SetVehicle (Utilities|ResolveSoftReference vehicle)))
  (Variables|Default|SetDriver (Utilities|ResolveSoftReference driver))
  (Pawn|Possess (Pawn|GetController _output_get) (Variables|Default|GetDriver)))

(fn SpawnVehiclenearby
  (Utilities|FindNearbyVehicle
    (:no%20vehicle%20found
      _)
    (:Found
      (return true))
    (:Vehicles%20Too%20Far%20Away
      _))
  (Utilities|SpawnNewVehicle)
  (return false))