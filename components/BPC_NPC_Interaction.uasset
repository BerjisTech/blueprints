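; NPC component that makes its owning character wander along the spline of the nearest actor tagged "pedestrian".
; A self-repeating short-delay loop, instead of Tick, finds the spline point closest to a velocity-derived trace hit and applies random-strength movement toward it, drawing a debug trace.
; BeginPlay also adds a scaled box collision to the owner, but its overlap handler is empty.
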(event Custom|random_walk
  (bind _character (Variables|Default|Getcharacter))
  (bind _returnvalue (Transformation|GetActorLocation _character))
  (bind _outactors (Actor|GetAllActorswithTag "pedestrian"))
  (Utilities|IsValid (Actor|GetComponentbyClass (.ReturnValue (Actor|FindNearestActor _returnvalue _outactors)) "/Script/Engine.SplineComponent")
    (:Is%20Valid
      (bind _outhit (Collision|LineTraceByChannel _returnvalue (Math|Vector|Normalize (+ (+ _returnvalue (* (Math|Vector|Normalize (Transformation|GetVelocity _character)) 5e+02)) 1e+01)) "TraceTypeQuery1" false 0 "None"))
      (Pawn|Input|AddMovementInput (Variables|Default|Getcharacter) (Math|Vector|GetUnitDirection(Vector) _returnvalue (Spline|FindLocationClosesttoWorldLocation (Actor|GetComponentbyClass (.ReturnValue (Actor|FindNearestActor _returnvalue _outactors)) "/Script/Engine.SplineComponent") (.location _outhit) "World")) (Math|Random|RandomFloatinRange 0.0 1.0) true)
      (Collision|LineTraceByChannel _returnvalue (Spline|FindLocationClosesttoWorldLocation (Actor|GetComponentbyClass (.ReturnValue (Actor|FindNearestActor _returnvalue _outactors)) "/Script/Engine.SplineComponent") (.location _outhit) "World") "TraceTypeQuery1" false 0 "ForDuration" true "(R=0.000000,G=0.025580,B=1.000000,A=1.000000)" "(R=0.942708,G=0.885417,B=1.000000,A=1.000000)")
      (Utilities|FlowControl|Delay 0.002)
      (CallFunction|RandomWalk))))

(event Custom|boxCollision
  (bind _returnvalue (Game|AddComponentbyClass (Components|GetOwner) "/Script/Engine.BoxComponent" false (Math|Transform|MakeTransform (Math|Vector|MakeVector 0.0 0.0 (.SphereRadius (Collision|GetComponentBounds (Variables|/Script/Engine.Character|GetMesh (Variables|Default|Getcharacter))))) "0, 0, 0" "4.000000,4.000000,1.000000")))
  (Collision|AssignOnComponentBeginOverlap _returnvalue (delegate Custom|OnComponentBeginOverlap_Event)))

(event Custom|OnComponentBeginOverlap_Event
  (params (OverlappedComponent :type Primitive%20Component%20Object%20Reference) (OtherActor :type Actor%20Object%20Reference) (OtherComp :type Primitive%20Component%20Object%20Reference) (OtherBodyIndex :type Integer) (bFromSweep :type Boolean) (SweepResult :type Hit%20Result%20Structure%20%28by%20ref%29)))

(event EventBeginPlay
  (bind _ascharacter (Utilities|Casting|CastToCharacter (Components|GetOwner)))
  (bind _output_get (Variables|Default|Setcharacter _ascharacter))
  (Variables|Default|Setmovement_component (Pawn|GetMovementComponent _output_get))
  (Variables|Default|Setcontroller (Pawn|GetController _ascharacter))
  (CallFunction|BoxCollision)
  (CallFunction|RandomWalk))

(event EventTick
  (params (DeltaSeconds :type Float%20%28single-precision%29)))