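; Mission manager component that loads the saved next mission from DT_Missions and runs its first unplayed objective on the matching level.
; After prerequisite checks, it places ground-traced markers, plays a sequence, shows the prompt, teleports the player, starts the HUD timer and spawns NPCs and vehicles.
; Marker overlaps check timing and dispatch by objective type, while Tick fails expired objectives.
; Type handlers, start/end calls and progress saving are stubs.
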(event Custom|getLastMission
  (bind _gameinstance (Variables|Default|GetgameInstance))
  (bind _currentgame (Variables|/Game/Blueprints/GameMode/SomboGameInstance.SomboGameInstance_C|GetcurrentGame _gameinstance))
  (Utilities|IsValid _gameinstance :!label _label
    (:Is%20Valid
      (Utilities|IsValid _currentgame :!label _label_2
        (:Is%20Valid
          (Variables|Default|SetnextMission (Utilities|String|StringToName (Utilities|String|EnumtoString (Variables|/Game/Blueprints/game_save/SG_PlayerData.SG_PlayerData_C|GetnextMission _currentgame))))
          (Variables|Default|SetcurrentMission (Utilities|String|StringToName (Utilities|String|EnumtoString (Variables|/Game/Blueprints/game_save/SG_PlayerData.SG_PlayerData_C|GetlastSavedMission _currentgame))))
          (CallFunction|MissionObjective (Variables|Default|GetnextMission)))
        (:Is%20Not%20Valid
          (Utilities|FlowControl|Delay 1.0)
          (goto _label_2))))
    (:Is%20Not%20Valid
      (Utilities|FlowControl|Delay 1.0)
      (goto _label))))

(event Custom|missionObjective
  (params (RowName :type Name))
  (bind _missionmarker (Variables|Default|GetmissionMarker))
  (bind _returnvalue (Utilities|GetDataTableRow "/Game/Blueprints/tables/DT_Missions.DT_Missions" RowName)
    (:then
      (bind _returnvalue_2 (Game|GetCurrentLevelName true))
      (if (Utilities|Enum|Equal(Enum) _returnvalue_2 (.missionlevel _returnvalue))
        (bind _output_get (Variables|Default|SetMissionObjectives (.missionobjectives _returnvalue)))
        (Variables|Default|SetcurrentlyPlaying (.mission _returnvalue))
        (Utilities|CheckifObjectiveHasBeenPlayed _output_get
          (:Completed
            (Variables|Default|SetactiveMissionObjective (.Value (Utilities|Map|Find _output_get (Variables|Default|GetcurrentObjective))))
            (Utilities|CheckPrequisiteMission
              (:Proceed
                (Utilities|CheckPrequisiteObjective
                  (:Proceed
                    (Utilities|PlaceMissionMarker)
                    (Utilities|ObjectiveSequence false)
                    (Utilities|DisplayPrompt)
                    (Utilities|ObjectiveStartLocation)
                    (Utilities|ObjectiveTimer true)
                    (Utilities|SpawnNPCs false
                      (:Completed
                        (Utilities|SpawnNPCVehicles false
                          (:true
                            (Utilities|SpawnNPCs true
                              (:Completed
                                (Utilities|SpawnNPCVehicles true
                                  (:true
                                    (Utilities|ObjectiveCall false
                                      (:true
                                        (bind _keys (Utilities|Map|Keys _missionmarker))
                                        (for _array_element _keys
                                          (EventDispatchers|AssignOnActorBeginOverlap (.Value (Utilities|Map|Find _missionmarker _array_element)) (delegate Custom|overlapMissionMarker)))))))))))))))))))))
    (:RowNotFound
      (Development|PrintString (Utilities|String|Append (Utilities|String|ToString(Name) RowName) " not found") true true "(R=0.000000,G=0.660000,B=1.000000,A=1.000000)" 2e+01))))

(event Custom|Rescue)

(event Custom|Kill)

(event Custom|Travel)

(event Custom|Collect)

(event Custom|overlapMissionMarker
  (params (OverlappedActor :type Actor%20Object%20Reference) (OtherActor :type Actor%20Object%20Reference))
  (bind _asbp_mission_marker (Utilities|Casting|CastToBP_MissionMarker OverlappedActor)
    (:then
      (Variables|Default|SetcurrentDestinatioon _asbp_mission_marker)
      (Utilities|HandleObjective)
      (Utilities|ObjectiveCall true
        (:true
          (Utilities|ObjectiveSequence true))))
    (:CastFailed
      (Development|PrintString "Hello"))))

(event Custom|Escort)

(event Custom|Deliver)

(event Custom|Race)

(event EventBeginPlay
  (Utilities|FlowControl|Delay 2.0)
  (if (Variables|/Game/Blueprints/GameMode/SomboGameInstance.SomboGameInstance_C|GetcanPlayMissions (Variables|Default|GetgameInstance))
    (CallFunction|GetLastMission)))

(event EventTick
  (params (DeltaSeconds :type Float%20%28single-precision%29))
  (Utilities|CheckTimer))