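; BP_PhysicsMeshSpawner is an actor that spawns BP_PhysicsMesh actors at its own transform with physics simulation enabled.
; Its SpawnMeshes event takes an index into the Meshes array, passes that mesh to the new actor and always spawns regardless of collision.
; A timed loop that would spawn random meshes is disconnected, and BeginPlay is empty, so nothing in this graph triggers spawning.
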(event Custom|Spawn%20Meshes
  (params (mesh%20index :type Integer))
  (bind _returnvalue (Game|SpawnActorfromClass "/Game/Blueprints/actor/BP_PhysicsMesh.BP_PhysicsMesh_C" (Transformation|GetActorTransform) "AlwaysSpawn" "MultiplyWithRoot" 0 (Utilities|Array|Get(acopy) (Variables|Default|Getmeshes) mesh%20index) 0))
  (Physics|SetSimulatePhysics (Variables|/Game/Blueprints/actor/BP_PhysicsMesh.BP_PhysicsMesh_C|GetStaticMesh _returnvalue) true))

(event EventBeginPlay)

(event Collision|EventActorBeginOverlap
  (params (OtherActor :type Actor%20Object%20Reference)))

(event EventTick
  (params (DeltaSeconds :type Float%20%28single-precision%29)))

(fn ConstructionScript)