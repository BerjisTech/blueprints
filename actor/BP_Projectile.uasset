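; BP_Projectile is a projectile actor that can home in on a target component.
; On BeginPlay, a valid HomingTargetComponent is passed to ProjectileMovement and the projectile self-destructs after a delay; without one, no lifetime timer starts.
; Box overlap with a non-Character destroys the projectile, then attempts a delayed destroy of the other actor, queued after self-destruction.
; A RadialForce impulse is present but unconnected.
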(event OnComponentBeginOverlap(Box)
  (params (OverlappedComponent :type Primitive%20Component%20Object%20Reference) (OtherActor :type Actor%20Object%20Reference) (OtherComp :type Primitive%20Component%20Object%20Reference) (OtherBodyIndex :type Integer) (bFromSweep :type Boolean) (SweepResult :type Hit%20Result%20Structure%20%28by%20ref%29))
  (if (not (Class|GameplayStatics|ObjectIsA OtherActor "/Script/Engine.Character"))
    (Actor|DestroyActor)
    (Utilities|FlowControl|Delay 1.0)
    (Actor|DestroyActor OtherActor)))

(event EventBeginPlay
  (bind _homing_target_component (Variables|Default|GetHoming%20Target%20Component))
  (Utilities|IsValid _homing_target_component
    (:Is%20Valid
      (Variables|/Script/Engine.ProjectileMovementComponent|SetHomingTargetComponent (Variables|Default|GetProjectileMovement) _homing_target_component)
      (Utilities|FlowControl|Delay 1e+01)
      (Actor|DestroyActor))))

(event Collision|EventActorBeginOverlap
  (params (OtherActor :type Actor%20Object%20Reference)))

(event EventTick
  (params (DeltaSeconds :type Float%20%28single-precision%29)))

(fn ConstructionScript)