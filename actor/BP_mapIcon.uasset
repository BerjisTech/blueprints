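; BP_mapIcon is a placeable mesh actor that can optionally act as a teleporter.
; The construction script toggles the mesh's visibility, and BeginPlay applies the custom mesh to it.
; When IsTeleporter is set, it binds the mesh's begin-overlap event at runtime, moving any overlapping actor straight to TeleportLocation without sweeping.
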(event Custom|updateMesh
  (Components|StaticMesh|SetStaticMesh (Variables|Default|GetSM_CylinderHollow) (Variables|Default|Getcustom_mesh))
  (CallFunction|Teleport))

(event Custom|Teleport
  (if (Variables|Default|Getis_teleporter)
    (Collision|AssignOnComponentBeginOverlap (Variables|Default|GetSM_CylinderHollow) (delegate Custom|OnComponentBeginOverlap_Event))))

(event Custom|OnComponentBeginOverlap_Event
  (params (OverlappedComponent :type Primitive%20Component%20Object%20Reference) (OtherActor :type Actor%20Object%20Reference) (OtherComp :type Primitive%20Component%20Object%20Reference) (OtherBodyIndex :type Integer) (bFromSweep :type Boolean) (SweepResult :type Hit%20Result%20Structure%20%28by%20ref%29))
  (Transformation|SetActorLocation OtherActor (Variables|Default|Getteleport_location) false true))

(event EventBeginPlay
  (CallFunction|UpdateMesh))

(event Collision|EventActorBeginOverlap
  (params (OtherActor :type Actor%20Object%20Reference)))

(event EventTick
  (params (DeltaSeconds :type Float%20%28single-precision%29)))

(fn ConstructionScript
  (Rendering|SetVisibility (Variables|Default|GetSM_CylinderHollow) (Variables|Default|Getshow_mesh) false))