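; Border actor that teleports any Character entering its Box to a point found behind them, apparently wrapping them across the map.
; On overlap, a very long trace against the character's forward vector finds the hit point, with persistent debug drawing.
; ShiftX selects whether X or Y passes through DynamiceAddReduce, whose 100-unit offset node is unconnected.
; A downward landscape trace from that point sets the final teleport location.
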(event OnComponentBeginOverlap(Box)
  (params (OverlappedComponent :type Primitive%20Component%20Object%20Reference) (OtherActor :type Actor%20Object%20Reference) (OtherComp :type Primitive%20Component%20Object%20Reference) (OtherBodyIndex :type Integer) (bFromSweep :type Boolean) (SweepResult :type Hit%20Result%20Structure%20%28by%20ref%29))
  (bind _returnvalue (Transformation|GetActorLocation OtherActor))
  (bind _shift_x (Variables|Default|Getshift_x))
  (if (Class|GameplayStatics|ObjectIsA OtherActor "/Script/Engine.Character")
    (bind _outhit (Collision|LineTraceByChannel _returnvalue (+ _returnvalue (* (Math|Vector|Normalize (Transformation|GetActorForwardVector OtherActor)) -2e+11)) "TraceTypeQuery3" true 0 "Persistent"))
    (bind _array_element_impact_point (CallFunction|LineTraceforLandscape (Math|Vector|MakeVector (Math|Float|SelectFloat (Utilities|DynamiceAddReduce (.x (.location _outhit))) (.x (.location _outhit)) _shift_x) (Math|Float|SelectFloat (.y (.location _outhit)) (Utilities|DynamiceAddReduce (.y (.location _outhit))) _shift_x) (.z (.location _outhit))) "0.000000,0.000000,-100000000.000000"))
    (Transformation|SetActorLocation OtherActor (Math|Vector|MakeVector (.x _array_element_impact_point) (.y _array_element_impact_point) (.z _array_element_impact_point)) false true)))

(event EventBeginPlay)

(event Collision|EventActorBeginOverlap
  (params (OtherActor :type Actor%20Object%20Reference)))

(event EventTick
  (params (DeltaSeconds :type Float%20%28single-precision%29)))

(fn ConstructionScript)