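; BP_PhysicsMesh is an actor that displays a configurable mesh and animates its vertical offset.
; BeginPlay assigns the mesh, caches the component's relative location and calls UpDown.
; UpDown plays the ZOffset timeline, adding its scaled track value to the cached Z without sweeping.
; Despite the name, no physics logic appears, and the ReverseUpDown branch has no effect on playback.
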(event Custom|UpDown
  (if (Variables|Default|GetreverseUpDown?)
    (bind _newtrack_0 (Timeline|ZOffset Play)
      (:Update
        (Transformation|SetRelativeLocation (Variables|Default|GetStaticMesh) (+ (Variables|Default|GetActorLocation) (Math|Vector|MakeVector 0.0 0.0 (* _newtrack_0 (Variables|Default|GetZOffset%20Factor)))) false false)))
    (else
      (Timeline|ZOffset Play))))

(event EventBeginPlay
  (Components|StaticMesh|SetStaticMesh (Variables|Default|GetStaticMesh) (Variables|Default|GetMesh))
  (Variables|Default|SetActorLocation (Variables|/Script/Engine.SceneComponent|GetRelativeLocation (Variables|Default|GetStaticMesh)))
  (CallFunction|UpDown))

(event Collision|EventActorBeginOverlap
  (params (OtherActor :type Actor%20Object%20Reference)))

(event EventTick
  (params (DeltaSeconds :type Float%20%28single-precision%29)))

(fn ConstructionScript)