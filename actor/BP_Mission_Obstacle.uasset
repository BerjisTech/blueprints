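; Mission obstacle actor that shows a configurable mesh and can spin it continuously.
; BeginPlay applies CustomMesh to the StaticMesh component and starts spinning when the Obstacle type is Spin.
; Spin eases the mesh's relative rotation toward an offset of SpinRotation with RInterpTo, then re-calls itself after a one-frame Delay instead of using Tick.
; The construction script's copy of this setup is disconnected, so it only takes effect at runtime.
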(event Custom|spin
  (bind _returnvalue (Utilities|Time|GetWorldDeltaSeconds))
  (bind _spin_rotation (Variables|Default|Getspin_rotation))
  (bind _staticmesh (Variables|Default|GetStaticMesh))
  (bind _relativerotation (Variables|/Script/Engine.SceneComponent|GetRelativeRotation _staticmesh))
  (bind (_roll _pitch _yaw) (Math|Rotator|BreakRotator _relativerotation))
  (Transformation|SetRelativeRotation (Variables|Default|GetStaticMesh) (Math|Interpolation|RInterpTo _relativerotation (Math|Rotator|MakeRotator (+ _roll (.roll _spin_rotation)) (+ _pitch (.pitch _spin_rotation)) (+ _yaw (.yaw _spin_rotation))) _returnvalue (Variables|Default|GetInterp%20Speed)) false true)
  (Utilities|FlowControl|Delay _returnvalue)
  (CallFunction|Spin))

(event EventBeginPlay
  (CallFunction|SetMesh)
  (switch Utilities|FlowControl|Switch|SwitchonENUM_Obstacle (Variables|Default|Getobstacle)
    (:NewEnumerator0
      (CallFunction|Spin))))

(event Collision|EventActorBeginOverlap
  (params (OtherActor :type Actor%20Object%20Reference)))

(event EventTick
  (params (DeltaSeconds :type Float%20%28single-precision%29)))

(fn ConstructionScript)

(fn SetMesh
  (Components|StaticMesh|SetStaticMesh (Variables|Default|GetStaticMesh) (Variables|Default|Getcustom_mesh)))