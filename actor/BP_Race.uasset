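; BP_Race runs a timed checkpoint race along RacePath, reporting the timer and win or timeout notices through PlayerHUD.
; Three reused cylinders show the upcoming checkpoints, grounded and oriented by a linear spline built from the path, with map icons respawned on each advance.
; Pawn overlap on the leading cylinder starts or advances the race, while a self-calling Delay loop polls for timeout.
; AddRacePoint appends the Arrow's transform to the path.
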(event OnComponentBeginOverlap(Cylinder)
  (params (OverlappedComponent :type Primitive%20Component%20Object%20Reference) (OtherActor :type Actor%20Object%20Reference) (OtherComp :type Primitive%20Component%20Object%20Reference) (OtherBodyIndex :type Integer) (bFromSweep :type Boolean) (SweepResult :type Hit%20Result%20Structure%20%28by%20ref%29))
  (if (Class|GameplayStatics|ObjectIsA OtherActor "/Script/Engine.Pawn")
    (if (== (Variables|Default|GetnextCheckpoint) 0)
      (CallFunction|StartRace))
    (Utilities|OutOfTime?
      (:No
        (Utilities|LastCheckpoint?
          (:Yes
            (Utilities|ClearCheckpoints)
            (Utilities|HUDNotice "YAY!!"))
          (:No
            (CallFunction|IncrementNextCheckpoint))))
      (:Yes
        (Utilities|ClearCheckpoints)
        (Utilities|HUDNotice "DND")))))

(event Custom|Spawn%20Checkpoints
  (bind _mapicons (Variables|Default|Getmapicons))
  (bind _racepath (Variables|Default|GetracePath))
  (for _array_element _mapicons
    (Actor|DestroyActor _array_element))
  (Utilities|Array|Clear _mapicons)
  (for _index (range 0 2)
    (bind _ground_location (CallFunction|PlaceonGround (.location (select (Utilities|Array|IsValidIndex _racepath (+ _index (Variables|Default|GetnextCheckpoint))) (Utilities|Array|Get(acopy) _racepath (+ _index (Variables|Default|GetnextCheckpoint))) (Math|Transform|MakeTransform "-1000000000000000.000000,-1000000000000000.000000,0.000000")))))
    (Transformation|SetWorldTransform (Utilities|Select :Index _index :Option%200 (Variables|Default|GetCylinder) :Option%201 (Variables|Default|GetCylinder1) :Option%202 (Variables|Default|GetCylinder2)) (Math|Transform|MakeTransform (+ _ground_location "0.000000,0.000000,50.000000") (Spline|GetRotationatSplinePoint (Variables|Default|GetSpline) (+ _index (Variables|Default|GetnextCheckpoint)) "World") (Transformation|GetWorldScale (Utilities|Select :Index _index :Option%200 (Variables|Default|GetCylinder) :Option%201 (Variables|Default|GetCylinder1) :Option%202 (Variables|Default|GetCylinder2)))) false true)
    (if (Utilities|Array|IsValidIndex _racepath (+ _index (Variables|Default|GetnextCheckpoint)))
      (bind _returnvalue (Game|SpawnActorfromClass "/Game/Blueprints/actor/BP_mapIcon.BP_mapIcon_C" (Math|Transform|MakeTransform (+ _ground_location "0.000000,0.000000,50.000000") "0, 0, 0" "0.100000,0.100000,0.100000") "Undefined" "MultiplyWithRoot" 0 (Utilities|Array|Get(acopy) (Variables|Default|GetMap%20Icon%20Texture) _index) "/Game/Blueprints/assets/StaticMesh/SM_CylinderHollow.SM_CylinderHollow" false "0.000000,0.000000,0.000000" true 0))
      (Utilities|Array|Add (Variables|Default|Getmapicons) _returnvalue))))

(event Custom|Add%20Race%20Point
  (Utilities|Array|Add (Variables|Default|GetracePath) (Transformation|GetWorldTransform (Variables|Default|GetArrow)))
  (CallFunction|IncrementNextCheckpoint))

(event Custom|Increment%20Next%20Checkpoint
  (Variables|Default|SetnextCheckpoint (+ (Variables|Default|GetnextCheckpoint) 1))
  (CallFunction|SpawnCheckpoints))

(event Custom|Start%20Race
  (Variables|Default|Setstart_time (Math|DateTime|Now))
  (Utilities|InitiateHUDTimer)
  (CallFunction|EllapsedTime))

(event Custom|Ellapsed%20Time
  (Variables|Default|Setellapsed_time (- (Math|DateTime|Now) (Variables|Default|Getstart_time)))
  (Utilities|OutOfTime?
    (:No
      (Utilities|FlowControl|Delay 0.002)
      (CallFunction|EllapsedTime))
    (:Yes
      (Utilities|ClearCheckpoints)
      (Utilities|HUDNotice "DND"))))

(event Custom|Draw%20Path
  (Utilities|Array|Clear (Variables|Default|GetsplinePoints))
  (for _array_element (Variables|Default|GetracePath)
    (Utilities|Array|Add (Variables|Default|GetsplinePoints) (.location _array_element)))
  (Spline|SetSplinePoints (Variables|Default|GetSpline) (Variables|Default|GetsplinePoints) "World" true)
  (for _index (range 0 (Spline|GetNumberOfSplinePoints (Variables|Default|GetSpline)))
    (Spline|SetSplinePointType (Variables|Default|GetSpline) _index "Linear" true)))

(event EventBeginPlay
  (bind _foundwidgets (Widget|GetAllWidgetsOfClass "/Game/Blueprints/widgets/MainMenus/PlayerHUD.PlayerHUD_C" true))
  (Variables|Default|SetHUD (Utilities|Array|Get(acopy) _foundwidgets))
  (CallFunction|DrawPath)
  (Variables|Default|SetnextCheckpoint 0)
  (CallFunction|SpawnCheckpoints))

(event Collision|EventActorBeginOverlap
  (params (OtherActor :type Actor%20Object%20Reference)))

(event EventTick
  (params (DeltaSeconds :type Float%20%28single-precision%29)))

(fn ConstructionScript)